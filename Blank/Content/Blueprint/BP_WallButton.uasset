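; BP_WallButton is an interactable wall button linked to a Door, with a text prompt that starts hidden.
; Its Box overlap toggles the prompt and BP_TestCharacter's CanInteract flag as the character enters and leaves.
; On entry it sets the character's InteractableActor to the Door rather than the button itself.
; A separate Interact_1 event on the button calls OpenDoor on the Door.
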(event `self.ReceiveBeginPlay`
  (`SceneComponent.SetHiddenInGame` (`self.TextRender`) true false))

(event `self.Box.OnComponentBeginOverlap`
  (params (OverlappedComponent :type "PrimitiveComponent Object Reference") (OtherActor :type "Actor Object Reference") (OtherComp :type "PrimitiveComponent Object Reference") (OtherBodyIndex :type Integer) (bFromSweep :type Boolean) (SweepResult :type "HitResult Structure (by ref)"))
  (bind _asbp_test_character (cast `/Game/Blueprint/BP_TestCharacter` OtherActor))
  (set `/Game/Blueprint/BP_TestCharacter.CanInteract` true _asbp_test_character)
  (set `/Game/Blueprint/BP_TestCharacter.InteractableActor` (`self.Door`) _asbp_test_character)
  (`SceneComponent.SetHiddenInGame` (`self.TextRender`) false false))

(event `self.Box.OnComponentEndOverlap`
  (params (OverlappedComponent :type "PrimitiveComponent Object Reference") (OtherActor :type "Actor Object Reference") (OtherComp :type "PrimitiveComponent Object Reference") (OtherBodyIndex :type Integer))
  (bind _asbp_test_character (cast `/Game/Blueprint/BP_TestCharacter` OtherActor))
  (set `/Game/Blueprint/BP_TestCharacter.CanInteract` false _asbp_test_character)
  (`SceneComponent.SetHiddenInGame` (`self.TextRender`) true false))

(event `Interact_1`
  (`InteractableDoor.OpenDoor` (`self.Door`)))

(fn `UserConstructionScript`)