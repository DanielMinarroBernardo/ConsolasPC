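; BP_ElevatingDoor is a door that rises once the player character has entered the correct password.
; A box overlap registers the door as the top-down character's interaction target and shows a prompt widget, clearing both on exit.
; The PuedeInteractuar event checks the player's PasswordAcertada flag, then plays a timeline that adds its track value to the cube's relative Z every update, so movement accumulates per frame.
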(event `self.Box.OnComponentBeginOverlap`
  (params (OverlappedComponent :type "PrimitiveComponent Object Reference") (OtherActor :type "Actor Object Reference") (OtherComp :type "PrimitiveComponent Object Reference") (OtherBodyIndex :type Integer) (bFromSweep :type Boolean) (SweepResult :type "HitResult Structure (by ref)"))
  (bind _asbp_top_down_character (cast `/Game/TopDown/Blueprints/BP_TopDownCharacter` OtherActor))
  (set `/Game/TopDown/Blueprints/BP_TopDownCharacter.OtherActor` self _asbp_top_down_character)
  (`SceneComponent.SetVisibility` (`self.Widget`) true false))

(event `self.Box.OnComponentEndOverlap`
  (params (OverlappedComponent :type "PrimitiveComponent Object Reference") (OtherActor :type "Actor Object Reference") (OtherComp :type "PrimitiveComponent Object Reference") (OtherBodyIndex :type Integer))
  (bind _asbp_top_down_character (cast `/Game/TopDown/Blueprints/BP_TopDownCharacter` OtherActor))
  (set `/Game/TopDown/Blueprints/BP_TopDownCharacter.OtherActor` null _asbp_top_down_character)
  (`SceneComponent.SetVisibility` (`self.Widget`) false false))

(event `/Game/Examen/BP_Interactua.PuedeInteractuar`
  (bind _asbp_top_down_character (cast `/Game/TopDown/Blueprints/BP_TopDownCharacter` (`GameplayStatics.GetPlayerCharacter` 0)))
  (if (`/Game/TopDown/Blueprints/BP_TopDownCharacter.PasswordAcertada` _asbp_top_down_character)
    (bind (_direction _newtrack_0) (`Timeline|Timeline`)
      (:`Update`
        (`SceneComponent.K2_AddRelativeLocation` (`self.Cube`) (`KismetMathLibrary.MakeVector` 0.0 0.0 _newtrack_0) false false)))))

(fn `UserConstructionScript`)