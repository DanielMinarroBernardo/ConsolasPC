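; BP_Key is an interactable key for a password puzzle, with its Key value displayed as text by the construction script.
; Box overlaps with BP_TopDownCharacter toggle a widget and set the character's OtherActor to this key, on both begin and end.
; PuedeInteractuar flashes the mesh red for a second, restores white, then sends Key and Tag to the BP_Password found at BeginPlay.
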(event `self.ReceiveBeginPlay`
  (bind _returnvalue (`GameplayStatics.GetActorOfClass` "/Game/Examen/BP_Password.BP_Password_C"))
  (set `self.TextRend` _returnvalue))

(event `self.Box.OnComponentBeginOverlap`
  (params (OverlappedComponent :type "PrimitiveComponent Object Reference") (OtherActor :type "Actor Object Reference") (OtherComp :type "PrimitiveComponent Object Reference") (OtherBodyIndex :type Integer) (bFromSweep :type Boolean) (SweepResult :type "HitResult Structure (by ref)"))
  (bind _asbp_top_down_character (cast `/Game/TopDown/Blueprints/BP_TopDownCharacter` OtherActor))
  (set `/Game/TopDown/Blueprints/BP_TopDownCharacter.OtherActor` self _asbp_top_down_character)
  (`SceneComponent.SetVisibility` (`self.Widget`) true false))

(event `self.Box.OnComponentEndOverlap`
  (params (OverlappedComponent :type "PrimitiveComponent Object Reference") (OtherActor :type "Actor Object Reference") (OtherComp :type "PrimitiveComponent Object Reference") (OtherBodyIndex :type Integer))
  (bind _asbp_top_down_character (cast `/Game/TopDown/Blueprints/BP_TopDownCharacter` OtherActor))
  (set `/Game/TopDown/Blueprints/BP_TopDownCharacter.OtherActor` self _asbp_top_down_character)
  (`SceneComponent.SetVisibility` (`self.Widget`) false false))

(event `/Game/Examen/BP_Interactua.PuedeInteractuar`
  (`PrimitiveComponent.SetMaterial` (`self.StaticMesh`) 0 "/Game/TopDown/Blueprints/MAT_Rojo.MAT_Rojo")
  (`KismetSystemLibrary.Delay` 1.0)
  (`PrimitiveComponent.SetMaterial` (`self.StaticMesh`) 0 "/Game/TopDown/Blueprints/MAT_Blanco.MAT_Blanco")
  (`/Game/Examen/BP_Interactua.SendNumber` (`self.TextRend`) (`self.Key`) (`self.Tag`)))

(fn `UserConstructionScript`
  (`TextRenderComponent.K2_SetText` (`self.TextRender`) (`self.Key`)))