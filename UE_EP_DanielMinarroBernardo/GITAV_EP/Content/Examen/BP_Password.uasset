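; Password keypad actor that displays typed input on a TextRender and checks it against the code stored on BP_TopDownCharacter.
; SendNumber branches on the key tag: numbers append to the text, C confirms, X clears.
; A correct entry prints a message and sets PasswordAcertada on the player cached at BeginPlay, while a wrong one clears the display.
; An unfinished loop over the player's ArrayPass is left disconnected.
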(event `self.ReceiveBeginPlay`
  (bind _asbp_top_down_character (cast `/Game/TopDown/Blueprints/BP_TopDownCharacter` (`GameplayStatics.GetPlayerCharacter` 0)))
  (set `self.My_Player` _asbp_top_down_character))

(event `/Game/Examen/BP_Interactua.SendNumber`
  (params (Key :type Text) (Tag :type "GameplayTag Structure"))
  (if (== Tag (struct :`TagName` "Key.number"))
    (bind _output_get (set `self.AcutalPassword` (`KismetTextLibrary.Conv_StringToText` (`KismetStringLibrary.Concat_StrStr` (`KismetTextLibrary.Conv_TextToString` (`self.AcutalPassword`)) (`KismetTextLibrary.Conv_TextToString` Key)))))
    (`TextRenderComponent.K2_SetText` (`self.TextRender`) _output_get)
    (elif (== Tag (struct :`TagName` "Key.c"))
      (if (== (`/Game/TopDown/Blueprints/BP_TopDownCharacter.Password` (`self.My_Player`)) (`KismetStringLibrary.Conv_StringToInt` (`KismetTextLibrary.Conv_TextToString` (`self.AcutalPassword`))))
        (`KismetSystemLibrary.PrintString` "acierto")
        (set `/Game/TopDown/Blueprints/BP_TopDownCharacter.PasswordAcertada` true (`self.My_Player`))
        (else
          (bind _output_get_2 (set `self.AcutalPassword` ""))
          (`TextRenderComponent.K2_SetText` (`self.TextRender`) _output_get_2)))
      (elif (== Tag (struct :`TagName` "Key.X"))
        (bind _output_get_3 (set `self.AcutalPassword` ""))
        (`TextRenderComponent.K2_SetText` (`self.TextRender`) _output_get_3)))))

(fn `UserConstructionScript`
  (`TextRenderComponent.K2_SetText` (`self.TextRender`) (`self.AcutalPassword`)))